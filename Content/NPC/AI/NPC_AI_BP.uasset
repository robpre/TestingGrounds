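; AI controller for patrolling guard NPCs that runs a guard behavior tree and feeds it perceived enemies.
; On BeginPlay it initializes the patrol blackboard, starts the tree and caches the controlled PatrollingGuard pawn.
; Perception updates are debug-printed, then set or clear the Enemy key for actors without the guard tag.
; Every tick, the guard's IsAiming flag mirrors whether the controller has a valid focus actor.
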(event OnTargetPerceptionUpdated(AIPerception)
  (params (Actor :type Actor%20Object%20Reference) (Stimulus :type AI%20Stimulus%20Structure))
  (bind _returnvalue (Utilities|Name|MakeLiteralName "Enemy"))
  (bind _activeblackboard (Variables|Default|GetActiveBlackboard))
  (bind (_actorout _stimulusout) (CallFunction|LogStimulusActivation Actor Stimulus))
  (if (not (Actor|ActorHasTag _actorout "guard"))
    (if (.bSuccessfullySensed (Utilities|Struct|BreakAIStimulus _stimulusout))
      (AI|Components|Blackboard|SetValueasObject _activeblackboard _returnvalue _actorout)
      (else
        (AI|Components|Blackboard|ClearValue _activeblackboard _returnvalue)))))

(event EventBeginPlay
  (bind _blackboardcomponent (Class|AIController|UseBlackboard "/Game/NPC/AI/PatrolData.PatrolData"))
  (Variables|Default|SetActiveBlackboard _blackboardcomponent)
  (AI|RunBehaviorTree "/Game/NPC/AI/GuardBehaviour.GuardBehaviour")
  (bind _aspatrolling_guard (Utilities|Casting|CastToPatrollingGuard (Pawn|GetControlledPawn)))
  (Variables|Default|SetPatrollingGuard _aspatrolling_guard))

(event EventTick
  (params (DeltaSeconds :type Float%20%28single-precision%29))
  (bind _patrollingguard (Variables|Default|GetPatrollingGuard))
  (Utilities|IsValid _patrollingguard
    (:Is%20Valid
      (Variables|/Game/NPC/Character/PatrollingGuard.PatrollingGuard_C|SetIsAiming _patrollingguard (Utilities|IsValid (Class|AIController|GetFocusActor))))))

(fn ConstructionScript)

(fn LogStimulusActivation
  (params (Actor :type Actor%20Object%20Reference) (Stimulus :type AI%20Stimulus%20Structure%20%28by%20ref%29))
  (bind (_age _expirationage) (Utilities|Struct|BreakAIStimulus Stimulus))
  (bind _returnvalue (Class|AIPerceptionSystem|GetSenseClassforStimulus Stimulus))
  (Development|PrintString (Utilities|String|Append (Utilities|GetObjectName (Pawn|GetControlledPawn)) " " (Utilities|GetClassDisplayName _returnvalue) " " (Utilities|GetDisplayName Actor) " " (Utilities|String|ToString(Float) _age) " " (Utilities|String|ToString(Float) _expirationage)))
  (return Actor Stimulus))